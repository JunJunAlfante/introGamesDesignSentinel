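; BP_Moving_Door is an actor that slides a static mesh door when something overlaps its Box trigger.
; On BeginPlay it stores the mesh's world location as the start point.
; Overlap plays a timeline whose Elevator track lerps the mesh toward that start plus a TargetLocation offset.
; Ending the overlap reverses the timeline, returning the door, with no filtering on the overlapping actor.
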(event OnComponentBeginOverlap(Box)
  (params (OverlappedComponent :type Primitive%20Component%20Object%20Reference) (OtherActor :type Actor%20Object%20Reference) (OtherComp :type Primitive%20Component%20Object%20Reference) (OtherBodyIndex :type Integer) (bFromSweep :type Boolean) (SweepResult :type Hit%20Result%20Structure%20%28by%20ref%29))
  (bind _startlocation (Variables|Default|GetstartLocation))
  (bind _elevator (Timeline|Timeline Play)
    (:Update
      (Transformation|SetWorldLocation (Variables|Default|GetStaticMesh) (Math|Vector|Lerp(Vector) _startlocation (+ _startlocation (Variables|Default|GettargetLocation)) _elevator) false false))))

(event OnComponentEndOverlap(Box)
  (params (OverlappedComponent :type Primitive%20Component%20Object%20Reference) (OtherActor :type Actor%20Object%20Reference) (OtherComp :type Primitive%20Component%20Object%20Reference) (OtherBodyIndex :type Integer))
  (bind _startlocation (Variables|Default|GetstartLocation))
  (bind _elevator (Timeline|Timeline Reverse)
    (:Update
      (Transformation|SetWorldLocation (Variables|Default|GetStaticMesh) (Math|Vector|Lerp(Vector) _startlocation (+ _startlocation (Variables|Default|GettargetLocation)) _elevator) false false))))

(event EventBeginPlay
  (Variables|Default|SetstartLocation (Transformation|GetWorldLocation (Variables|Default|GetStaticMesh))))

(event Collision|EventActorBeginOverlap
  (params (OtherActor :type Actor%20Object%20Reference)))

(event EventTick
  (params (DeltaSeconds :type Float%20%28single-precision%29)))

(fn ConstructionScript)