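; BP_SignPost_Zone1 is a Zone 1 signpost actor that shows a text widget while something overlaps its sphere.
; On BeginPlay it hides the Widget component, casts its user widget to WBP_SignPost_Zone1 and passes TextToShow through UpdateSignpost.
; The sphere's begin and end overlap events toggle the widget's visibility, with no check on which actor triggers them.
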(event OnComponentBeginOverlap(Sphere)
  (params (OverlappedComponent :type Primitive%20Component%20Object%20Reference) (OtherActor :type Actor%20Object%20Reference) (OtherComp :type Primitive%20Component%20Object%20Reference) (OtherBodyIndex :type Integer) (bFromSweep :type Boolean) (SweepResult :type Hit%20Result%20Structure%20%28by%20ref%29))
  (Rendering|SetVisibility (Variables|Default|GetWidget) true false))

(event OnComponentEndOverlap(Sphere)
  (params (OverlappedComponent :type Primitive%20Component%20Object%20Reference) (OtherActor :type Actor%20Object%20Reference) (OtherComp :type Primitive%20Component%20Object%20Reference) (OtherBodyIndex :type Integer))
  (Rendering|SetVisibility (Variables|Default|GetWidget) false false))

(event EventBeginPlay
  (Rendering|SetVisibility (Variables|Default|GetWidget) false false)
  (bind _aswbp_sign_post_zone_1 (Utilities|Casting|CastToWBP_SignPost_Zone1 (UserInterface|GetUserWidgetObject (Variables|Default|GetWidget))))
  (Default|UpdateSignpost _aswbp_sign_post_zone_1 (Variables|Default|GetTextToShow)))

(event Collision|EventActorBeginOverlap
  (params (OtherActor :type Actor%20Object%20Reference)))

(event EventTick
  (params (DeltaSeconds :type Float%20%28single-precision%29)))

(fn ConstructionScript)