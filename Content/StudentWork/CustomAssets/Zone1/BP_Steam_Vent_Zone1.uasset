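; BP_Steam_Vent_Zone1 is a Zone 1 steam vent hazard that also acts as a trigger for a linked door and sign.
; Overlapping its box starts a looping timer that repeatedly damages the overlapping actor, opens MyDoor and sets MySign's text to show the door is open.
; Ending the overlap clears the timer and closes the door, but leaves the sign text unchanged.
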(event OnComponentEndOverlap(Box)
  (params (OverlappedComponent :type Primitive%20Component%20Object%20Reference) (OtherActor :type Actor%20Object%20Reference) (OtherComp :type Primitive%20Component%20Object%20Reference) (OtherBodyIndex :type Integer))
  (Variables|Default|Settriggered false)
  (Utilities|Time|ClearandInvalidateTimerbyHandle (Variables|Default|GetTimer))
  (Default|CloseDoor (Variables|Default|GetMy%20Door)))

(event OnComponentBeginOverlap(Box)
  (params (OverlappedComponent :type Primitive%20Component%20Object%20Reference) (OtherActor :type Actor%20Object%20Reference) (OtherComp :type Primitive%20Component%20Object%20Reference) (OtherBodyIndex :type Integer) (bFromSweep :type Boolean) (SweepResult :type Hit%20Result%20Structure%20%28by%20ref%29))
  (Variables|Default|Settriggered true)
  (bind _returnvalue (Utilities|Time|SetTimerbyEvent (delegate Custom|PainMaker) 0.2 true))
  (Variables|Default|SetTimer _returnvalue)
  (Default|OpenDoor (Variables|Default|GetMy%20Door))
  (Variables|/Game/StudentWork/CustomAssets/Zone1/BP_SignPost_Zone1.BP_SignPost_Zone1_C|SetTextToShow (Variables|Default|GetMy%20Sign) "DOOR OPEN"))

(event Custom|PainMaker
  (Game|Damage|ApplyDamage (stale OnComponentBeginOverlap(Box) OtherActor) 3.0 0 0))

(event EventBeginPlay)

(event Collision|EventActorBeginOverlap
  (params (OtherActor :type Actor%20Object%20Reference)))

(event EventTick
  (params (DeltaSeconds :type Float%20%28single-precision%29)))

(fn ConstructionScript)