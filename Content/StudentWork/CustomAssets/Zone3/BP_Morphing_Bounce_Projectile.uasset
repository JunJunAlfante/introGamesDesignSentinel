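; BP_Morphing_Bounce_Projectile is a projectile that changes size over time and damages actors that overlap it.
; On BeginPlay it stores the Sphere's world scale, then a Timeline lerps SphereCollision's world scale from that value to EndSize.
; Each SphereCollision overlap applies fixed damage and prints a debug "BOUNCE", but only a PlayerCharacter overlap destroys the projectile.
; An unconnected radius-lerp node never runs.
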(event OnComponentBeginOverlap(SphereCollision)
  (params (OverlappedComponent :type Primitive%20Component%20Object%20Reference) (OtherActor :type Actor%20Object%20Reference) (OtherComp :type Primitive%20Component%20Object%20Reference) (OtherBodyIndex :type Integer) (bFromSweep :type Boolean) (SweepResult :type Hit%20Result%20Structure%20%28by%20ref%29))
  (Game|Damage|ApplyDamage OtherActor 5.0 0 0)
  (Development|PrintString "BOUNCE")
  (Utilities|Casting|CastToPlayerCharacter OtherActor)
  (Actor|DestroyActor))

(event EventBeginPlay
  (Variables|Default|SetstartSize (Transformation|GetWorldScale (Variables|Default|GetSphere)))
  (bind _sizemorphingovertime (Timeline|Timeline Play)
    (:Update
      (Transformation|SetWorldScale3D (Variables|Default|GetSphereCollision) (Math|Vector|Lerp(Vector) (Variables|Default|GetstartSize) (Variables|Default|GetendSize) _sizemorphingovertime)))))

(event Collision|EventActorBeginOverlap
  (params (OtherActor :type Actor%20Object%20Reference)))

(event EventTick
  (params (DeltaSeconds :type Float%20%28single-precision%29)))

(fn ConstructionScript)