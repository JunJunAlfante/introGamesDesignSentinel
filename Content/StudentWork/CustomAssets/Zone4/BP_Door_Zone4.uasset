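; BP_Door_Zone4 is a door actor for Zone 4 that slides open and closed through its OpenDoor and CloseDoor events.
; On BeginPlay it records the static mesh's world location as the closed position.
; A timeline's Door track drives a lerp from that start to the start plus a TargetLocation offset, and CloseDoor reverses the same timeline to return it.
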(event Custom|Open%20Door
  (bind _startlocation (Variables|Default|GetstartLocation))
  (bind _door (Timeline|Timeline Play)
    (:Update
      (Transformation|SetWorldLocation (Variables|Default|GetStaticMesh) (Math|Vector|Lerp(Vector) _startlocation (+ _startlocation (Variables|Default|GettargetLocation)) _door) false false))))

(event Custom|Close%20Door
  (bind _startlocation (Variables|Default|GetstartLocation))
  (bind _door (Timeline|Timeline Reverse)
    (:Update
      (Transformation|SetWorldLocation (Variables|Default|GetStaticMesh) (Math|Vector|Lerp(Vector) _startlocation (+ _startlocation (Variables|Default|GettargetLocation)) _door) false false))))

(event EventBeginPlay
  (Variables|Default|SetstartLocation (Transformation|GetWorldLocation (Variables|Default|GetStaticMesh))))

(event Collision|EventActorBeginOverlap
  (params (OtherActor :type Actor%20Object%20Reference)))

(event EventTick
  (params (DeltaSeconds :type Float%20%28single-precision%29)))

(fn ConstructionScript)