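; BP_Key_Zone4 is a damage-activated switch actor that opens and closes a set of linked doors in Zone 4.
; Any damage flips its Triggered flag, then it calls OpenDoor or CloseDoor on each valid entry in MyDoors to match the new state.
; It has no other active logic; BeginPlay, overlap, Tick and the construction script are empty.
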(event EventBeginPlay)

(event Collision|EventActorBeginOverlap
  (params (OtherActor :type Actor%20Object%20Reference)))

(event EventTick
  (params (DeltaSeconds :type Float%20%28single-precision%29)))

(event Game|Damage|EventAnyDamage
  (params (Damage :type Float%20%28single-precision%29) (DamageType :type Damage%20Type%20Object%20Reference) (InstigatedBy :type Controller%20Object%20Reference) (DamageCauser :type Actor%20Object%20Reference))
  (bind _mydoors (Variables|Default|GetMyDoors))
  (if (Variables|Default|GetTriggered)
    (Variables|Default|SetTriggered false)
    (for _array_element _mydoors
      (Utilities|IsValid _array_element
        (:Is%20Valid
          (Default|CloseDoor _array_element))))
    (else
      (Variables|Default|SetTriggered true)
      (for _array_element_2 _mydoors
        (Utilities|IsValid _array_element_2
          (:Is%20Valid
            (Default|OpenDoor _array_element_2)))))))

(fn ConstructionScript)