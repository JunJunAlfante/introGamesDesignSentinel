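; Moving platform that rises and lowers while the ControlUp and ControlDown components are overlapped, stopping when overlap ends.
; Two timelines lerp Platform between its BeginPlay world location and vertical or in/out offsets, applied as relative location.
; In/out and rotation events have no callers here; rotation events set fixed StaticMesh roll angles.
; Hits on the clockwise and anticlockwise controls only toggle a Rotating flag, which drives no rotation.
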(event OnComponentBeginOverlap(ControlUp)
  (params (OverlappedComponent :type Primitive%20Component%20Object%20Reference) (OtherActor :type Actor%20Object%20Reference) (OtherComp :type Primitive%20Component%20Object%20Reference) (OtherBodyIndex :type Integer) (bFromSweep :type Boolean) (SweepResult :type Hit%20Result%20Structure%20%28by%20ref%29))
  (CallFunction|MoveUp))

(event OnComponentEndOverlap(ControlUp)
  (params (OverlappedComponent :type Primitive%20Component%20Object%20Reference) (OtherActor :type Actor%20Object%20Reference) (OtherComp :type Primitive%20Component%20Object%20Reference) (OtherBodyIndex :type Integer))
  (CallFunction|StopUpDown))

(event OnComponentBeginOverlap(ControlDown)
  (params (OverlappedComponent :type Primitive%20Component%20Object%20Reference) (OtherActor :type Actor%20Object%20Reference) (OtherComp :type Primitive%20Component%20Object%20Reference) (OtherBodyIndex :type Integer) (bFromSweep :type Boolean) (SweepResult :type Hit%20Result%20Structure%20%28by%20ref%29))
  (CallFunction|MoveDown))

(event OnComponentEndOverlap(ControlDown)
  (params (OverlappedComponent :type Primitive%20Component%20Object%20Reference) (OtherActor :type Actor%20Object%20Reference) (OtherComp :type Primitive%20Component%20Object%20Reference) (OtherBodyIndex :type Integer))
  (CallFunction|StopUpDown))

(event OnComponentHit(ControlClockwise)
  (params (HitComponent :type Primitive%20Component%20Object%20Reference) (OtherActor :type Actor%20Object%20Reference) (OtherComp :type Primitive%20Component%20Object%20Reference) (NormalImpulse :type Vector :default "0, 0, 0") (Hit :type Hit%20Result%20Structure%20%28by%20ref%29))
  (if (Variables|Default|GetRotating)
    (Variables|Default|SetRotating false)
    (else
      (Variables|Default|SetRotating true))))

(event OnComponentHit(ControlAnticlockwise)
  (params (HitComponent :type Primitive%20Component%20Object%20Reference) (OtherActor :type Actor%20Object%20Reference) (OtherComp :type Primitive%20Component%20Object%20Reference) (NormalImpulse :type Vector :default "0, 0, 0") (Hit :type Hit%20Result%20Structure%20%28by%20ref%29))
  (if (Variables|Default|GetRotating)
    (Variables|Default|SetRotating false)
    (else
      (Variables|Default|SetRotating true))))

(event Custom|Move%20In
  (bind _maxout (Variables|Default|GetMaxOut))
  (bind _movement (Timeline|Timeline_0 Play)
    (:Update
      (Transformation|SetRelativeLocationAndRotation (Variables|Default|GetPlatform) (Math|Vector|Lerp(Vector) _maxout (+ _maxout (Variables|Default|GetMaxIn)) _movement) "0, 0, 0" false false))))

(event Custom|Move%20Out
  (bind _maxout (Variables|Default|GetMaxOut))
  (bind _movement (Timeline|Timeline_0 Reverse)
    (:Update
      (Transformation|SetRelativeLocationAndRotation (Variables|Default|GetPlatform) (Math|Vector|Lerp(Vector) _maxout (+ _maxout (Variables|Default|GetMaxIn)) _movement) "0, 0, 0" false false))))

(event Custom|Rotate%20AntiClockwise
  (Transformation|SetWorldRotation (Variables|Default|GetStaticMesh) (Math|Rotator|MakeRotator (Variables|Default|GetAntiClockwise) 0.0 0.0) false false))

(event Custom|StopRotation
  (Transformation|SetWorldRotation (Variables|Default|GetStaticMesh) (Math|Rotator|MakeRotator 0.0 0.0 0.0) false false))

(event Custom|Move%20Up
  (bind _maxdown (Variables|Default|GetMaxDown))
  (bind _movement (Timeline|Timeline Play)
    (:Update
      (Transformation|SetRelativeLocationAndRotation (Variables|Default|GetPlatform) (Math|Vector|Lerp(Vector) _maxdown (+ _maxdown (Variables|Default|GetMaxUp)) _movement) "0, 0, 0" false false))))

(event Custom|Move%20Down
  (bind _maxdown (Variables|Default|GetMaxDown))
  (bind _movement (Timeline|Timeline Reverse)
    (:Update
      (Transformation|SetRelativeLocationAndRotation (Variables|Default|GetPlatform) (Math|Vector|Lerp(Vector) _maxdown (+ _maxdown (Variables|Default|GetMaxUp)) _movement) "0, 0, 0" false false))))

(event Custom|StopUpDown
  (bind _maxdown (Variables|Default|GetMaxDown))
  (bind _movement (Timeline|Timeline Stop)
    (:Update
      (Transformation|SetRelativeLocationAndRotation (Variables|Default|GetPlatform) (Math|Vector|Lerp(Vector) _maxdown (+ _maxdown (Variables|Default|GetMaxUp)) _movement) "0, 0, 0" false false))))

(event Custom|StopInOut
  (bind _maxout (Variables|Default|GetMaxOut))
  (bind _movement (Timeline|Timeline_0 Stop)
    (:Update
      (Transformation|SetRelativeLocationAndRotation (Variables|Default|GetPlatform) (Math|Vector|Lerp(Vector) _maxout (+ _maxout (Variables|Default|GetMaxIn)) _movement) "0, 0, 0" false false))))

(event Custom|Rotate%20Clockwise
  (Transformation|SetWorldRotation (Variables|Default|GetStaticMesh) (Math|Rotator|MakeRotator (Variables|Default|GetClockwise) 0.0 0.0) false false))

(event Collision|EventActorBeginOverlap
  (params (OtherActor :type Actor%20Object%20Reference)))

(event EventTick
  (params (DeltaSeconds :type Float%20%28single-precision%29)))

(event EventBeginPlay
  (bind _platform (Variables|Default|GetPlatform))
  (bind _returnvalue (Transformation|GetWorldLocation _platform))
  (Variables|Default|SetMaxDown _returnvalue)
  (Variables|Default|SetMaxOut _returnvalue))

(fn ConstructionScript)