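; BP_Auto_Double_Door is an automatic double door that slides open when something overlaps its Box and closes when an overlap ends.
; BeginPlay caches both door meshes' world locations as start points.
; Overlap plays or reverses a Timeline, whose LeftDoor track drives both doors' lerps toward start plus per-door TargetLocation offsets in world space.
; Overlaps are not filtered by actor or counted.
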(event OnComponentBeginOverlap(Box)
  (params (OverlappedComponent :type Primitive%20Component%20Object%20Reference) (OtherActor :type Actor%20Object%20Reference) (OtherComp :type Primitive%20Component%20Object%20Reference) (OtherBodyIndex :type Integer) (bFromSweep :type Boolean) (SweepResult :type Hit%20Result%20Structure%20%28by%20ref%29))
  (bind _startlocationright (Variables|Default|GetstartLocationRight))
  (bind _startlocationleft (Variables|Default|GetstartLocationLeft))
  (bind _left_door (Timeline|Timeline Play)
    (:Update
      (Transformation|SetWorldLocation (Variables|Default|GetSM_DoorLeft) (Math|Vector|Lerp(Vector) _startlocationleft (+ _startlocationleft (Variables|Default|GettargetLocationLeft)) _left_door) false false)
      (Transformation|SetWorldLocation (Variables|Default|GetSM_DoorRight) (Math|Vector|Lerp(Vector) _startlocationright (+ _startlocationright (Variables|Default|GettargetLocationRight)) _left_door) false false))))

(event OnComponentEndOverlap(Box)
  (params (OverlappedComponent :type Primitive%20Component%20Object%20Reference) (OtherActor :type Actor%20Object%20Reference) (OtherComp :type Primitive%20Component%20Object%20Reference) (OtherBodyIndex :type Integer))
  (bind _startlocationright (Variables|Default|GetstartLocationRight))
  (bind _startlocationleft (Variables|Default|GetstartLocationLeft))
  (bind _left_door (Timeline|Timeline Reverse)
    (:Update
      (Transformation|SetWorldLocation (Variables|Default|GetSM_DoorLeft) (Math|Vector|Lerp(Vector) _startlocationleft (+ _startlocationleft (Variables|Default|GettargetLocationLeft)) _left_door) false false)
      (Transformation|SetWorldLocation (Variables|Default|GetSM_DoorRight) (Math|Vector|Lerp(Vector) _startlocationright (+ _startlocationright (Variables|Default|GettargetLocationRight)) _left_door) false false))))

(event EventBeginPlay
  (Variables|Default|SetstartLocationLeft (Transformation|GetWorldLocation (Variables|Default|GetSM_DoorLeft)))
  (Variables|Default|SetstartLocationRight (Transformation|GetWorldLocation (Variables|Default|GetSM_DoorRight))))

(event Collision|EventActorBeginOverlap
  (params (OtherActor :type Actor%20Object%20Reference)))

(event EventTick
  (params (DeltaSeconds :type Float%20%28single-precision%29)))

(fn ConstructionScript)