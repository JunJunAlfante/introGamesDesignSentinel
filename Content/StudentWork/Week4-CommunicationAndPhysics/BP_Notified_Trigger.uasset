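; Trigger actor that toggles a referenced door whenever its static mesh registers a hit.
; A DoorOpen flag picks between calling OpenDoor and CloseDoor on MyDoor and flips with each hit.
; On the first opening only, a DoOnce gate spawns a WBP_PickUpNotification actor at the trigger's location to announce that the door opened.
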(event OnComponentHit(StaticMesh)
  (params (HitComponent :type Primitive%20Component%20Object%20Reference) (OtherActor :type Actor%20Object%20Reference) (OtherComp :type Primitive%20Component%20Object%20Reference) (NormalImpulse :type Vector :default "0, 0, 0") (Hit :type Hit%20Result%20Structure%20%28by%20ref%29))
  (if (Variables|Default|GetDoorOpen)
    (Default|CloseDoor (Variables|Default|GetMyDoor))
    (Variables|Default|SetDoorOpen false)
    (else
      (Default|OpenDoor (Variables|Default|GetMyDoor))
      (Variables|Default|SetDoorOpen true)
      (Utilities|FlowControl|DoOnce false
        (:Completed
          (Game|SpawnActorfromClass "/Game/UI/WBP_PickUpNotification.WBP_PickUpNotification_C" (Math|Transform|MakeTransform (.location (Transformation|GetActorTransform)) "0, 0, 0" "1.000000,1.000000,1.000000") "Undefined" "MultiplyWithRoot" 0 "Door Opened!" 0))))))

(event EventBeginPlay)

(event Collision|EventActorBeginOverlap
  (params (OtherActor :type Actor%20Object%20Reference)))

(event EventTick
  (params (DeltaSeconds :type Float%20%28single-precision%29)))

(fn ConstructionScript)