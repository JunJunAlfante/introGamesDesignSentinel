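; BP_Trigger_Multi is a trigger actor that opens or closes several doors at once when its static mesh is hit.
; Each hit on the mesh flips a DoorOpen flag, so successive hits alternate between closing and opening.
; It loops over the MyDoor array and calls OpenDoor or CloseDoor on every valid entry, skipping invalid references.
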(event OnComponentHit(StaticMesh)
  (params (HitComponent :type Primitive%20Component%20Object%20Reference) (OtherActor :type Actor%20Object%20Reference) (OtherComp :type Primitive%20Component%20Object%20Reference) (NormalImpulse :type Vector :default "0, 0, 0") (Hit :type Hit%20Result%20Structure%20%28by%20ref%29))
  (if (Variables|Default|GetDoorOpen)
    (Variables|Default|SetDoorOpen false)
    (for _array_element (Variables|Default|GetMyDoor)
      (Utilities|IsValid _array_element
        (:Is%20Valid
          (Default|CloseDoor _array_element))))
    (else
      (Variables|Default|SetDoorOpen true)
      (for _array_element_2 (Variables|Default|GetMyDoor)
        (Utilities|IsValid _array_element_2
          (:Is%20Valid
            (Default|OpenDoor _array_element_2)))))))

(event EventBeginPlay)

(event Collision|EventActorBeginOverlap
  (params (OtherActor :type Actor%20Object%20Reference)))

(event EventTick
  (params (DeltaSeconds :type Float%20%28single-precision%29)))

(fn ConstructionScript)