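; BP_Moving_Turret is a turret actor that starts moving and firing automatically on BeginPlay.
; A timeline lerps it from its starting location toward that point plus the TargetLocation offset, without sweeping.
; A second timeline's Fire event track spawns a BP_Projectile at the Arrow component's world location and rotation.
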(event Custom|Turret%20Fires
  (bind _arrow (Variables|Default|GetArrow))
  (bind _returnvalue (Transformation|GetWorldTransform _arrow))
  (Game|SpawnActorfromClass "/Game/StudentWork/Week5-ProjectilesAndExtras/BP_Projectile.BP_Projectile_C" (Math|Transform|MakeTransform (.location _returnvalue) (.rotation _returnvalue) "1.000000,1.000000,1.000000") "Undefined" "MultiplyWithRoot" 0 0))

(event Custom|Turret%20Infinite%20Fires
  (Timeline|TurretFiresTL Play
    (:Fire
      (CallFunction|TurretFires))))

(event Custom|Turret%20Moving
  (Variables|Default|SetstartLocation (Transformation|GetActorLocation))
  (bind _movingtl (Timeline|Timeline Play)
    (:Update
      (Transformation|SetActorLocation (Math|Vector|Lerp(Vector) (Variables|Default|GetstartLocation) (+ (Variables|Default|GetstartLocation) (Variables|Default|GettargetLocation)) _movingtl) false false))))

(event EventBeginPlay
  (CallFunction|TurretMoving)
  (CallFunction|TurretInfiniteFires))

(event Collision|EventActorBeginOverlap
  (params (OtherActor :type Actor%20Object%20Reference)))

(event EventTick
  (params (DeltaSeconds :type Float%20%28single-precision%29)))

(fn ConstructionScript)