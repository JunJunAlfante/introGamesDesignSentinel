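; BP_Dummy is a damageable target dummy actor with an on-screen health bar carried by a widget component.
; On BeginPlay it caches the component's WBP_DummyHealth widget.
; AnyDamage prints a pain message, subtracts from current health, pushes the fraction of an assumed 100 maximum to the bar, and destroys the actor at zero or below.
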(event EventBeginPlay
  (bind _aswbp_dummy_health (Utilities|Casting|CastToWBP_DummyHealth (UserInterface|GetUserWidgetObject (Variables|Default|GetWidget))))
  (Variables|Default|SetDummy%20Health%20Bar _aswbp_dummy_health))

(event Collision|EventActorBeginOverlap
  (params (OtherActor :type Actor%20Object%20Reference)))

(event EventTick
  (params (DeltaSeconds :type Float%20%28single-precision%29)))

(event Game|Damage|EventAnyDamage
  (params (Damage :type Float%20%28single-precision%29) (DamageType :type Damage%20Type%20Object%20Reference) (InstigatedBy :type Controller%20Object%20Reference) (DamageCauser :type Actor%20Object%20Reference))
  (Development|PrintString "Ow!")
  (bind _output_get (Variables|Default|SetCurrentHealth (- (Variables|Default|GetCurrentHealth) Damage)))
  (Default|UpdateHealth (Variables|Default|GetDummy%20Health%20Bar) (/ _output_get 1e+02))
  (if (<= (Variables|Default|GetCurrentHealth) 0.0)
    (Actor|DestroyActor)))

(fn ConstructionScript)